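; Display platform actor for an animation showcase, with a title that names the animation it presents.
; The construction script uses the PlatformSize setting to pick the mesh, move the title to the platform edge and scale the animation-detection box.
; The title shows OverrideName if set, otherwise the Animation asset's name with underscores and the first five characters removed.
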(fn `Initialize_Platform`
  (bind _override_name (`self.Override_Name`))
  (bind _animation (`self.Animation`))
  (bind _returnvalue (select `/Game/MorroMotion(RE)/Platforms/EPlatformSize` (`self.Platform_Size`) :`NewEnumerator0` 250.0 :`NewEnumerator1` 350.0 :`NewEnumerator2` 450.0 :`NewEnumerator3` 550.0 :!type "Float (single-precision)"))
  ;[0 0 0] Set platform size and title location
  (`StaticMeshComponent.SetStaticMesh` (`self.SM_Platform`) (select `/Game/MorroMotion(RE)/Platforms/EPlatformSize` (`self.Platform_Size`) :`NewEnumerator0` "/Game/MorroMotion(RE)/Platforms/Mesh/SM_Platform_Small.SM_Platform_Small" :`NewEnumerator1` "/Game/MorroMotion(RE)/Platforms/Mesh/SM_Platform_Medium.SM_Platform_Medium" :`NewEnumerator2` "/Game/MorroMotion(RE)/Platforms/Mesh/SM_Platform_Large.SM_Platform_Large" :`NewEnumerator3` "/Game/MorroMotion(RE)/Platforms/Mesh/SM_Platform_XLarge.SM_Platform_XLarge" :!type "StaticMesh Object Reference")) ; Set platform to appropriate size.
  (`SceneComponent.K2_SetRelativeLocation` (`self.TextRender_Title`) (`KismetMathLibrary.MakeVector` (select `/Game/MorroMotion(RE)/Platforms/EPlatformSize` (`self.Platform_Size`) :`NewEnumerator0` -255.0 :`NewEnumerator1` -355.0 :`NewEnumerator2` -455.0 :`NewEnumerator3` -555.0 :!type "Float (single-precision)")) false false) ; Set title location to edge of platform.
  (`BoxComponent.SetBoxExtent` (`self.Box`) (`KismetMathLibrary.MakeVector` _returnvalue _returnvalue 25.0) true) ; Set extent of box for animation detection.
  ;[0 0 0] If "Override_Name" is set, use it
  (if (`KismetTextLibrary.TextIsEmpty` _override_name)
    ;[0 0 0] If "Animation" is valid, set the Title to the animation name
    (`/Engine/EditorBlueprintResources/StandardMacros.IsValid` _animation
      (:`Is Valid`
        (`TextRenderComponent.K2_SetText` (`self.TextRender_Title`) (`KismetTextLibrary.Conv_StringToText` (`KismetStringLibrary.RightChop` (`KismetStringLibrary.Replace` (`KismetSystemLibrary.GetDisplayName` _animation) "_" " ") 5)))))
    (else
      (`TextRenderComponent.K2_SetText` (`self.TextRender_Title`) _override_name))))

(fn `UserConstructionScript`
  (`self.Initialize_Platform`))