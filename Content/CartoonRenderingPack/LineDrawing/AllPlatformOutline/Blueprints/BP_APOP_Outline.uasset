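; Outline component that gives its owning actor an outline by overlaying copies of its visible skeletal and static meshes.
; On BeginPlay it spawns an attached, collision-free mesh actor for each visible mesh component and applies LineMaterial to every material slot.
; Skeletal copies follow the source animation through master pose.
; Spawned actors are tracked in AttachedOutlineActors and destroyed when the owner is destroyed.
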(event Custom|Event%20Destory%20OutlineActors
  ;[1 1 1] Handle Destroying actor
  (for _array_element (Variables|Default|GetAttachedOutlineActors)
    (Actor|DestroyActor _array_element)))

(event EventBeginPlay
  ;[1 1 1] Variable setup: OwnerActor
  (bind _output_get (Variables|Default|SetOwner%20Actor (Components|GetOwner)))
  ;[1 1 1] Handle Destroying actor
  (Game|BindEventtoOnDestroyed _output_get (delegate Custom|Event%20Destory%20OutlineActors))
  ;[1 1 1] Generate outlines for all skeletal mesh components
  (for _array_element (Actor|GetComponentsByClass (Variables|Default|GetOwner%20Actor) "/Script/Engine.SkeletalMeshComponent")
    (CallFunction|GenSkeletalMeshComponentOutline _array_element))
  ;[1 1 1] Generate outlines for static mesh components
  (for _array_element_2 (Actor|GetComponentsByClass (Variables|Default|GetOwner%20Actor) "/Script/Engine.StaticMeshComponent")
    (CallFunction|GenStaticMeshComponentOutline _array_element_2)))

(fn GenSkeletalMeshComponentOutline
  (params (SkeletalMeshComponent :type Skeletal%20Mesh%20Component%20Object%20Reference))
  ;[1 1 1] Variable setup: TargetSkeletalMeshComponent, TargetSkeletalMesh
  (bind _output_get (LocalVariables|SetTargetSkeletalMeshComponent SkeletalMeshComponent))
  (LocalVariables|SetTargetSkeletalMesh (Variables|/Script/Engine.SkinnedMeshComponent|GetSkeletalMesh _output_get))
  ;[1 1 1] Filter only visible mesh components
  (if (Rendering|IsVisible (LocalVariables|GetTargetSkeletalMeshComponent))
    ;[1 1 1] Create a line mesh actor and component by duplicating the owner actor, and transform it the same to the owner actor
    (bind _returnvalue (Game|SpawnActorfromClass "/Script/Engine.SkeletalMeshActor" (Transformation|GetActorTransform (Variables|Default|GetOwner%20Actor)) "AlwaysSpawn" 0 0))
    ;[1 1 1] VariableSetup: SkeletalLineMeshActor, SkeletalLineMeshComponent
    (bind _output_get_2 (LocalVariables|SetSkeletalLineMeshActor _returnvalue))
    (LocalVariables|SetSkeletalLineMeshComponent (Variables|/Script/Engine.SkeletalMeshActor|GetSkeletalMeshComponent _output_get_2))
    ;[1 1 1] Add the new actor to the attached actors array
    (Utilities|Array|Add (Variables|Default|GetAttachedOutlineActors) (LocalVariables|GetSkeletalLineMeshActor))
    ;[1 1 1] Snap the line mesh actor to the owner actor
    (Class|Actor|AttachRootComponenttoActor (LocalVariables|GetSkeletalLineMeshActor) (Variables|Default|GetOwner%20Actor) "None" "KeepRelativeOffset" true)
    (Transformation|SetWorldTransform (LocalVariables|GetSkeletalLineMeshComponent) (Transformation|GetWorldTransform (LocalVariables|GetTargetSkeletalMeshComponent)) false false)
    ;[1 1 1] Set the owner actor's skeletal mesh to the line mesh component
    (Class|SkinnedMeshComponent|SetSkeletalMesh (LocalVariables|GetSkeletalLineMeshComponent) (LocalVariables|GetTargetSkeletalMesh))
    ;[1 1 1] Disable collision for the line mesh
    (Collision|SetCollisionEnabled (LocalVariables|GetSkeletalLineMeshComponent) "NoCollision")
    ;[1 1 1] Set owner actor's the animation blueprint to the line mesh component.
    (Class|SkinnedMeshComponent|SetMasterPoseComponent (LocalVariables|GetSkeletalLineMeshComponent) (LocalVariables|GetTargetSkeletalMeshComponent))
    ;[1 1 1] Set the selected line material to all elements of the line mesh component
    (for (_ _array_index) (Rendering|Material|GetMaterials (LocalVariables|GetSkeletalLineMeshComponent))
      (Rendering|Material|SetMaterial (LocalVariables|GetSkeletalLineMeshComponent) _array_index (Variables|Default|GetLineMaterial)))
    (return)
    (else
      (return))))

(fn GenStaticMeshComponentOutline
  (params (StaticMeshComponent :type Static%20Mesh%20Component%20Object%20Reference))
  (bind _owner_actor (Variables|Default|GetOwner%20Actor))
  ;[1 1 1] VariableSetup: TargetStaticMeshComponent, TargetStaticMesh
  (bind _output_get (LocalVariables|SetTargetStaticMeshComponent StaticMeshComponent))
  (LocalVariables|SetTargetStaticMesh (Variables|/Script/Engine.StaticMeshComponent|GetStaticMesh _output_get))
  ;[1 1 1] Filter only visible meshes
  (if (Rendering|IsVisible (LocalVariables|GetTargetStaticMeshComponent))
    ;[1 1 1] Create a line mesh actor by duplicating the owner actor, and transform it the same to the owner actor
    (Game|SpawnActorfromClass "/Game/CartoonRenderingPack/LineDrawing/AllPlatformOutline/Blueprints/SM_APOP_Dummy.SM_APOP_Dummy_C" (Transformation|GetActorTransform _owner_actor) "AlwaysSpawn" _owner_actor 0)
    ;[1 1 1] VariableSetup: StaticLineMeshActor, StaticLineMeshComponent
    (bind _output_get_2 (LocalVariables|SetStaticLineMeshActor 0))
    (LocalVariables|SetStaticLineMeshComponent (Variables|/Script/Engine.StaticMeshActor|GetStaticMeshComponent _output_get_2))
    ;[1 1 1] Add the new actor to the attached actors array
    (Utilities|Array|Add (Variables|Default|GetAttachedOutlineActors) (LocalVariables|GetStaticLineMeshActor))
    ;[1 1 1] Snap the line mesh actor to the owner actor
    (Class|Actor|AttachRootComponenttoActor (LocalVariables|GetStaticLineMeshActor) (Variables|Default|GetOwner%20Actor) "None" "SnapToTargetIncludingScale" true)
    (Transformation|SetWorldTransform (LocalVariables|GetStaticLineMeshComponent) (Transformation|GetWorldTransform (LocalVariables|GetTargetStaticMeshComponent)) false false)
    ;[1 1 1] Set the owner actor's static mesh to the line mesh component
    (Components|StaticMesh|SetStaticMesh (LocalVariables|GetStaticLineMeshComponent) (LocalVariables|GetTargetStaticMesh))
    ;[1 1 1] Disable collision for the line mesh
    (Collision|SetCollisionEnabled (LocalVariables|GetStaticLineMeshComponent) "NoCollision")
    ;[1 1 1] Set the selected line material to all elements of the line mesh component
    (for (_ _array_index) (Rendering|Material|GetMaterials (LocalVariables|GetStaticLineMeshComponent))
      (Rendering|Material|SetMaterial (LocalVariables|GetStaticLineMeshComponent) _array_index (Variables|Default|GetLineMaterial)))
    (return)
    (else
      (return))))