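; Player Blueprint that handles input for hitting notes and interacting with widgets in an idol-themed game.
; The HitNote action notifies NoteControlCenter on press and also drives a WidgetInteraction component as a left mouse press and release.
; The P key asks IdolGameMode to change its UI state, and BeginPlay turns on the FPS stat display.
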(event `self.ReceiveBeginPlay`
  (`KismetSystemLibrary.ExecuteConsoleCommand` "Stat FPS" null))

(event `InputAction|HitNote`
  (params (Key :type "Key Structure"))
  (bind _widgetinteraction (`self.WidgetInteraction`))
  (:`Pressed`
    (`/Game/Blueprint/NotesSystem/NoteControlCenter.ButtonPressed` (`self.NoteControlCenter`))
    (`WidgetInteractionComponent.PressPointerKey` _widgetinteraction "LeftMouseButton"))
  (:`Released`
    (`WidgetInteractionComponent.ReleasePointerKey` _widgetinteraction "LeftMouseButton")))

(event `Key|P`
  (params (Key :type "Key Structure"))
  (:`Pressed`
    (bind _asidol_game_mode (cast `/Game/Blueprint/System/IdolGameMode` (`GameplayStatics.GetGameMode`)))
    (`/Game/Blueprint/System/IdolGameMode.ChangeUIState` _asidol_game_mode "NewEnumerator0")))

(fn `UserConstructionScript`)