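; IdolGameMode is the game mode for a VR music game, switching between the Ready and Game Start UI states.
; BeginPlay caches the Player_VR pawn and stops the audio.
; ChangeUIState shows the pawn's tagged MainWidget with query collision and stops audio in Ready.
; In Game Start it hides the widget, disables its collision, plays audio and calls MusicStart on the note controller reference supplied through GetREF.
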(event `self.ReceiveBeginPlay`
  (bind _asplayer_vr (cast `/Game/Blueprint/Player/Player_VR` (`GameplayStatics.GetPlayerPawn` 0)))
  (set `self.Player` _asplayer_vr)
  (`AudioComponent.Stop` (`self.Audio`)))

(event `ChangeUIState`
  (params (UIState :type "/Game/Blueprint/UI/UIState Enum" :default "NewEnumerator0"))
  (bind _output_get (set `self.UIState` UIState))
  (switch `/Game/Blueprint/UI/UIState` _output_get
    (:`NewEnumerator0`
      (bind _aswidget_component (cast `WidgetComponent` (`|GetArrayItem` (`self.GetComponentsByTag` (`self.Player`) "/Script/Engine.ActorComponent" "MainWidget"))))
      (`SceneComponent.SetVisibility` _aswidget_component true false)
      (`PrimitiveComponent.SetCollisionEnabled` _aswidget_component "QueryOnly")
      (`AudioComponent.Stop` (`self.Audio`)))
    (:`NewEnumerator2`
      (bind _aswidget_component_2 (cast `WidgetComponent` (`|GetArrayItem` (`self.GetComponentsByTag` (`self.Player`) "/Script/Engine.ActorComponent" "MainWidget"))))
      (`SceneComponent.SetVisibility` _aswidget_component_2 false false)
      (`PrimitiveComponent.SetCollisionEnabled` _aswidget_component_2 "NoCollision")
      (`AudioComponent.Play` (`self.Audio`) 0.0)
      (`/Game/Blueprint/NotesSystem/NoteControlCenter.MusicStart` (`self.NOTE_CONTROL_REF`)))))

(event `GetREF`
  (params (REF :type "/Game/Blueprint/NotesSystem/NoteControlCenter Object Reference"))
  (set `self.NOTE_CONTROL_REF` REF))

(fn `UserConstructionScript`)