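; Rhythm-game note controller that spawns, judges and retires two lanes of music notes.
; BeginPlay loads note times and lanes from a data table, registers with IdolGameMode and pre-spawns a note pool per lane.
; Once music starts, Tick shows pooled notes ahead of their hit time and hides overdue ones as misses.
; F or ButtonPressed grades timing as Perfect, Great or Miss, triggering score displays and particles.
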(event `self.ReceiveBeginPlay`
  (bind _const_note_max_n (`self.CONST_NOTE_MAX_N`))
  (`self.EnableInput` (`GameplayStatics.GetPlayerController` 0))
  (bind _asidol_game_mode (cast `/Game/Blueprint/System/IdolGameMode` (`GameplayStatics.GetGameMode`)))
  (set `self.GameMode` _asidol_game_mode)
  ;[1 1 1] NoteDataLoad
  (bind _returnvalue (`DataTableFunctionLibrary.GetDataTableColumnAsString` "/Game/ExternalData/NoteData.NoteData" "NoteTimePassed"))
  (for _array_element _returnvalue
    (`KismetArrayLibrary.Array_Add` (`self.NoteTimePassedLocal`) (`KismetStringLibrary.Conv_StringToInt` _array_element)))
  (bind _returnvalue_2 (`DataTableFunctionLibrary.GetDataTableColumnAsString` "/Game/ExternalData/NoteData.NoteData" "NotePosition"))
  (for _array_element_2 _returnvalue_2
    (`KismetArrayLibrary.Array_Add` (`self.NotePositionLocal`) (`KismetStringLibrary.Conv_StringToInt` _array_element_2)))
  (`/Game/Blueprint/System/IdolGameMode.GetREF` (`self.GameMode`) self)
  (`self.NotePoolingFunc` 0 _const_note_max_n)
  (`self.NotePoolingFunc` 1 _const_note_max_n))

(event `Key|X`
  (params (Key :type "Key Structure"))
  ;[1 1 1] MusicStart (Variable Initialize)
  (:`Pressed`
    (set `self.MusicStartTime` (`KismetMathLibrary.Now`) :!label _label)
    (set `self.GameOn` true)
    (set `self.SpawnedNoteIndex` 0)
    (set `self.ToBePressdIndex` 0)))

(event `MusicStart`
  ;[1 1 1] MusicStart (Variable Initialize)
  (goto _label))

(event `MusicStop`
  ;[1 1 1] MusicStop
  (set `self.GameOn` false))

(event `self.ReceiveTick`
  (params (DeltaSeconds :type "Float (single-precision)"))
  (if (`self.GameOn`)
    (`|ExecutionSequence`
      (:`then_0`
        ;[1 1 1] Is Time To Spawn?
        (bind _output (`self.MillToTimeSpan` (`|GetArrayItem` (`self.NoteTimePassedLocal`) (`self.SpawnedNoteIndex`))))
        (if (< (- (+ (`self.MusicStartTime`) _output) (`self.Delay`)) (`KismetMathLibrary.Now`))
          (`self.SpawnNote`)))
      (:`then_1`
        ;[1 1 1] Kill OverTimed Note
        (bind _output_2 (`self.MillToTimeSpan` (`|GetArrayItem` (`self.NoteTimePassedLocal`) (`self.ToBePressdIndex`))))
        (if (> (- (`KismetMathLibrary.Now`) (+ (`self.MusicStartTime`) _output_2)) (`self.DeleteTime`))
          (`self.KillNote`)
          (`self.ShowScore` 2))))))

(event `Key|F`
  (params (Key :type "Key Structure"))
  (bind _returnvalue (`self.K2_GetActorLocation` (`self.CenterPosition`)))
  ;[1 1 1] Key Input
  (:`Pressed`
    (bind _presstimedifference (`self.TimeDifferenceCheck` :!label _label_2))
    (set `self.TempTime` _presstimedifference)
    (if (<= _presstimedifference (`self.PerfectTime`))
      (`self.ShowScore` 0)
      (`GameplayStatics.SpawnEmitterAtLocation` "/Game/UI/Particle/Shine2.Shine2" _returnvalue)
      (`self.KillNote` :!label _label_3)
      (elif (<= (`self.TempTime`) (`self.GreatTime`))
        (`self.ShowScore` 1)
        (`GameplayStatics.SpawnEmitterAtLocation` "/Game/UI/Particle/Shine2.Shine2" _returnvalue)
        (goto _label_3)
        (elif (<= (`self.TempTime`) (`self.MissTime`))
          (`self.ShowScore` 2)
          (`GameplayStatics.SpawnEmitterAtLocation` "/Game/UI/Particle/Shine2.Shine2" _returnvalue)
          (goto _label_3))))))

(event `ButtonPressed`
  ;[1 1 1] Key Input
  (goto _label_2))

(fn `KillNote`
  (bind _rightindextoberemoved (`self.RightIndexToBeRemoved`))
  (bind _leftindextoberemoved (`self.LeftIndexToBeRemoved`))
  (bind _const_note_max_n (`self.CONST_NOTE_MAX_N`))
  (switch `int` (`|GetArrayItem` (`self.NotePositionLocal`) (`self.ToBePressdIndex`))
    (:`0`
      (`/Game/Blueprint/NotesSystem/MusicNoteParent.SET NOT VISIBLE` (`|GetArrayItem` (`self.MusicNoteRight`) _rightindextoberemoved))
      (bind _result (`/Engine/EditorBlueprintResources/StandardMacros.IncrementInt` _rightindextoberemoved)
        (:`  `
          (if (== _result _const_note_max_n)
            (set `self.RightIndexToBeRemoved` 0)))))
    (:`1`
      (`/Game/Blueprint/NotesSystem/MusicNoteParent.SET NOT VISIBLE` (`|GetArrayItem` (`self.MusicNoteLeft`) _leftindextoberemoved))
      (bind _result_2 (`/Engine/EditorBlueprintResources/StandardMacros.IncrementInt` _leftindextoberemoved)
        (:`  `
          (if (== _result_2 _const_note_max_n)
            (set `self.LeftIndexToBeRemoved` 0))))))
  (`/Engine/EditorBlueprintResources/StandardMacros.IncrementInt` (`self.ToBePressdIndex`)))

(fn `MillToTimeSpan`
  (params (MillSec :type Integer))
  (returns (OutPut :type "Timespan Structure"))
  (bind (_remainder _returnvalue) (`KismetMathLibrary.FMod` (`KismetMathLibrary.Conv_IntToDouble` MillSec) 1000.0))
  (bind (_remainder_2 _returnvalue_2) (`KismetMathLibrary.FMod` (`KismetMathLibrary.Conv_IntToDouble` _returnvalue) 60.0))
  (return (`KismetMathLibrary.MakeTimespan` 0 0 _returnvalue_2 (`KismetMathLibrary.FTrunc` _remainder_2) (`KismetMathLibrary.FTrunc` _remainder))))

(fn `NotePoolingFunc`
  (params (`0or1` :type Integer) (MakeNum :type Integer))
  (for _ (range (+ MakeNum 1))
    (bind _returnvalue (`|SpawnActorFromClass` (`|GetArrayItem` (`self.NoteNumber`) `0or1`) (`KismetMathLibrary.MakeTransform` (`SceneComponent.K2_GetComponentLocation` (`Actor.RootComponent` (`|GetArrayItem` (`self.NotePositionActor`) `0or1`))) (struct :`Yaw` 180.0)) "Undefined" "OverrideRootScale" null null))
    (bind _asmusic_note_parent (cast `/Game/Blueprint/NotesSystem/MusicNoteParent` _returnvalue))
    (switch `int` `0or1`
      (:`0`
        (`KismetArrayLibrary.Array_Add` (`self.MusicNoteRight`) _asmusic_note_parent))
      (:`1`
        (`KismetArrayLibrary.Array_Add` (`self.MusicNoteLeft`) _asmusic_note_parent))))
  (return))

(fn `ScoreUIKiller`)

(fn `ShowScore`
  (params (Perfect0Great1Miss2 :type Integer))
  (bind _scoreperfect (`self.ScorePerfect`))
  (bind _scoregreat (`self.ScoreGreat`))
  (bind _scoremiss (`self.ScoreMiss`))
  (bind _defaultsceneroot (`/Game/UI/BP/ScoreParent.DefaultSceneRoot` _scoremiss))
  (bind _defaultsceneroot_2 (`/Game/UI/BP/ScoreParent.DefaultSceneRoot` _scoregreat))
  (bind _defaultsceneroot_3 (`/Game/UI/BP/ScoreParent.DefaultSceneRoot` _scoreperfect))
  (switch `int` Perfect0Great1Miss2
    (:`0`
      (`SceneComponent.SetVisibility` _defaultsceneroot true true)
      (`SceneComponent.SetVisibility` _defaultsceneroot_3 true true)
      (`/Game/UI/BP/ScoreParent.AnimationReset` _scoreperfect)
      (`SceneComponent.SetVisibility` _defaultsceneroot_2 false true)
      (`SceneComponent.SetVisibility` _defaultsceneroot false true)
      (`/Game/Blueprint/NotesSystem/NoteControlInterface.KillHim` _scoremiss)
      (`/Game/Blueprint/NotesSystem/NoteControlInterface.KillHim` _scoreperfect))
    (:`1`
      (`SceneComponent.SetVisibility` _defaultsceneroot_2 true true)
      (`/Game/UI/BP/ScoreParent.AnimationReset` _scoregreat)
      (`SceneComponent.SetVisibility` _defaultsceneroot_3 false true)
      (`SceneComponent.SetVisibility` _defaultsceneroot false true)
      (`/Game/Blueprint/NotesSystem/NoteControlInterface.KillHim` _scoregreat))
    (:`2`
      (`SceneComponent.SetVisibility` _defaultsceneroot true true)
      (`/Game/UI/BP/ScoreParent.AnimationReset` _scoremiss)
      (`SceneComponent.SetVisibility` _defaultsceneroot_3 false true)
      (`SceneComponent.SetVisibility` _defaultsceneroot_2 false true)
      (`/Game/Blueprint/NotesSystem/NoteControlInterface.KillHim` _scoremiss))))

(fn `SpawnNote`
  (bind _leftindex (`self.LEFTINDEX`))
  (bind _rightindex (`self.RIGHTINDEX`))
  (switch `int` (`|GetArrayItem` (`self.NotePositionLocal`) (`self.SpawnedNoteIndex`))
    (:`0`
      (`/Game/Blueprint/NotesSystem/MusicNoteParent.SET VISIBLE` (`|GetArrayItem` (`self.MusicNoteRight`) _rightindex))
      (bind _result (`/Engine/EditorBlueprintResources/StandardMacros.IncrementInt` _rightindex)
        (:`  `
          (if (== _result 10)
            (set `self.RIGHTINDEX` 0)))))
    (:`1`
      (`/Game/Blueprint/NotesSystem/MusicNoteParent.SET VISIBLE` (`|GetArrayItem` (`self.MusicNoteLeft`) _leftindex))
      (bind _result_2 (`/Engine/EditorBlueprintResources/StandardMacros.IncrementInt` _leftindex)
        (:`  `
          (if (== _result_2 10)
            (set `self.LEFTINDEX` 0))))))
  (`/Engine/EditorBlueprintResources/StandardMacros.IncrementInt` (`self.SpawnedNoteIndex`)))

(fn `TimeDifferenceCheck`
  (returns (PressTimeDifference :type "Timespan Structure"))
  (bind _returnvalue (`KismetMathLibrary.Now`))
  (bind _output (`self.MillToTimeSpan` (`|GetArrayItem` (`self.NoteTimePassedLocal`) (`self.ToBePressdIndex`))))
  (bind _returnvalue_2 (+ (`self.MusicStartTime`) _output))
  (if (>= _returnvalue _returnvalue_2)
    (return (- _returnvalue _returnvalue_2))
    (else
      (return (- _returnvalue_2 _returnvalue)))))

(fn `UserConstructionScript`)